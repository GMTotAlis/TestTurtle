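; First-person test character with movement, camera look and interaction with in-world buttons.
; Every tick, a short camera line trace finds actors implementing Interact_Interface_BP and shows their select message in a Butten_Widget created at BeginPlay, clearing it otherwise.
; The Button Pressed graph receives the hit actor and combines the E key with two boolean flags to send InteractMessage once per press.
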(event `InputAxis|Move Forward/Backward`
  (params (AxisValue :type "Float (single-precision)"))
  ;[1 1 1] Character movement
  (`self.AddMovementInput` (`KismetMathLibrary.GetForwardVector` (`KismetMathLibrary.MakeRotator` 0.0 0.0 (.yaw (`self.GetControlRotation`)))) AxisValue))

(event `InputAxis|Move Right/Left`
  (params (AxisValue :type "Float (single-precision)"))
  ;[1 1 1] Character movement
  (`self.AddMovementInput` (`KismetMathLibrary.GetRightVector` (`KismetMathLibrary.MakeRotator` 0.0 0.0 (.yaw (`self.GetControlRotation`)))) AxisValue))

(event `InputAxis|Look Up/Down`
  (params (AxisValue :type "Float (single-precision)"))
  ;[1 1 1] Rotation camera
  (`self.AddControllerPitchInput` AxisValue))

(event `InputAxis|Look Right/Left`
  (params (AxisValue :type "Float (single-precision)"))
  ;[1 1 1] Rotation camera
  (`self.AddControllerYawInput` AxisValue))

(event `self.ReceiveBeginPlay`
  ;[1 1 1] Add viewport when begin play
  (bind _returnvalue (`|CreateWidget` "/Game/Blueprints/Butten_Widget.Butten_Widget_C"))
  (bind _output_get (set `self.Select REF` _returnvalue))
  (`UserWidget.AddToViewport` _output_get 0))

(event `Select Button`
  (bind _camera (`self.Camera`))
  (bind _returnvalue (`SceneComponent.K2_GetComponentLocation` _camera))
  ;[1 1 1] Button select and press controll
  ;;[1 1 1] Check is camera look in button
  (bind (_outhit _returnvalue_2) (`KismetSystemLibrary.LineTraceSingle` _returnvalue (+ _returnvalue (* (`SceneComponent.GetForwardVector` _camera) 150.0)) "TraceTypeQuery1"))
  ;;[1 1 1] If camera look at button then put text in viewport, else put nothing
  (if _returnvalue_2
    (bind (_bblockinghit _binitialoverlap _time _distance _location _impactpoint _normal _impactnormal _physmat _hitactor) (`GameplayStatics.BreakHitResult` _outhit))
    (if (`KismetSystemLibrary.DoesImplementInterface` _hitactor "/Game/Blueprints/Interact_Interface_BP.Interact_Interface_BP_C")
      (bind _selected_button (message `/Game/Blueprints/Interact_Interface_BP.Get Select` _hitactor))
      (set `/Game/Blueprints/Butten_Widget.Selected Button` _selected_button (`self.Select REF`))
      (set `self.Is Proseed` true)
      (if (and (`self.Is Pressed`) (`self.Is Proseed`)) :!label _label
        (set `self.Is Proseed` false)
        (set `self.Is Pressed` false)
        (message `/Game/Blueprints/Interact_Interface_BP.Interact` _hitactor self))
      (else
        (set `/Game/Blueprints/Butten_Widget.Selected Button` "" (`self.Select REF`) :!label _label_2)))
    (else
      (goto _label_2))))

(event `Key|E`
  (params (Key :type "Key Structure"))
  ;[1 1 1] Button select and press controll
  (:`Pressed`
    (set `self.Is Pressed` true)
    (goto _label)))

(event `self.ReceiveTick`
  (params (DeltaSeconds :type "Float (single-precision)"))
  (`self.Select Button`))

(fn `UserConstructionScript`)