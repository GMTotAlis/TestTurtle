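; Automatic sliding door Blueprint that opens when a Turtle_Bot_BP enters its box trigger and closes when it leaves.
; Overlap events play the Open or Close component and run the Doors timeline forward or in reverse.
; The timeline output, scaled by Distance, drives OpenTheDoor, which slides left and right panels apart along X and the top panel along Z.
; BeginPlay resets all three panels to zero relative location.
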(event `self.ReceiveBeginPlay`
  (`SceneComponent.K2_SetRelativeLocation` (`self.D_Left`) (0.0 0.0 0.0) false false)
  (`SceneComponent.K2_SetRelativeLocation` (`self.D_Right`) (0.0 0.0 0.0) false false)
  (`SceneComponent.K2_SetRelativeLocation` (`self.D_Top`) (0.0 0.0 0.0) false false))

(event `self.Box.OnComponentBeginOverlap`
  (params (OverlappedComponent :type "PrimitiveComponent Object Reference") (OtherActor :type "Actor Object Reference") (OtherComp :type "PrimitiveComponent Object Reference") (OtherBodyIndex :type Integer) (bFromSweep :type Boolean) (SweepResult :type "HitResult Structure (by ref)"))
  (cast `/Game/Blueprints/Turtle/Turtle_Bot_BP` OtherActor)
  (`AudioComponent.Play` (`self.Open`) 0.0)
  (bind (_direction _newtrack_0) (`Timeline|Doors` :!label _label)
    (:`Update`
      (`self.Open_The_Door` (* _newtrack_0 (`self.distance`))))))

(event `self.Box.OnComponentEndOverlap`
  (params (OverlappedComponent :type "PrimitiveComponent Object Reference") (OtherActor :type "Actor Object Reference") (OtherComp :type "PrimitiveComponent Object Reference") (OtherBodyIndex :type Integer))
  (cast `/Game/Blueprints/Turtle/Turtle_Bot_BP` OtherActor)
  (`AudioComponent.Play` (`self.Close`) 0.0)
  (goto _label :!via `Reverse`))

(fn `Open_The_Door`
  (params (distance :type "Float (double-precision)"))
  (`|ExecutionSequence`
    (:`then_0`
      ;[1 1 1] Left Slider
      (`SceneComponent.K2_SetRelativeLocation` (`self.D_Left`) (`KismetMathLibrary.MakeVector` (* -1 distance)) false false))
    (:`then_1`
      ;[1 1 1] Right Slider
      (`SceneComponent.K2_SetRelativeLocation` (`self.D_Right`) (`KismetMathLibrary.MakeVector` distance) false false))
    (:`then_2`
      ;[1 1 1] Top Slider
      (`SceneComponent.K2_SetRelativeLocation` (`self.D_Top`) (`KismetMathLibrary.MakeVector` 0.0 0.0 distance) false false))))

(fn `UserConstructionScript`)