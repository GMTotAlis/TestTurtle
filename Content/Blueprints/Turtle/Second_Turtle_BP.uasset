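; Second turtle Blueprint that moves in a stop-and-go rhythm along its movement direction.
; While IsMoving is true, Tick calls MoveTurtle with direction scaled by speed and delta time.
; Two Delay nodes on Tick toggle the flag, giving about one second of movement and a half-second pause.
; The construction script only calls the parent's version.
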(event `self.ReceiveTick`
  (params (DeltaSeconds :type "Float (single-precision)"))
  (if (`self.Is Moving`)
    (`self.Move Turtle` (* (`self.Movement Direction`) (* DeltaSeconds (`self.Speed`))))
    (`KismetSystemLibrary.Delay` 1.0)
    (set `self.Is Moving` false)
    (else
      (`KismetSystemLibrary.Delay` 0.5)
      (set `self.Is Moving` true))))

(fn `UserConstructionScript`
  (`parent.UserConstructionScript`))