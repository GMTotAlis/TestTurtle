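; Third turtle Blueprint that moves back and forth along MovementDirection, spending longer going forward than backward.
; Each Tick calls MoveTurtle with a step scaled by Speed and DeltaSeconds, negated when IsMovingForward is false.
; Delay nodes on each Tick branch time the flip of IsMovingForward, giving about one second forward and half a second back.
; The construction script only calls its parent.
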(event `self.ReceiveTick`
  (params (DeltaSeconds :type "Float (single-precision)"))
  (bind _returnvalue (* DeltaSeconds (`self.Speed`)))
  (if (`self.Is Moving Forward`)
    (`self.Move Turtle` (* (`self.Movement Direction`) _returnvalue))
    (`KismetSystemLibrary.Delay` 1.0)
    (set `self.Is Moving Forward` false)
    (else
      (`self.Move Turtle` (* (* (`self.Movement Direction`) -1) _returnvalue))
      (`KismetSystemLibrary.Delay` 0.5)
      (set `self.Is Moving Forward` true))))

(fn `UserConstructionScript`
  (`parent.UserConstructionScript`))