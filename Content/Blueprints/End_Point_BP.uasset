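; End point actor that removes turtles when they reach it and plays a burn effect.
; A box overlap casts the other actor to Turtle_BP, then destroys it after a short delay.
; It then plays Burn, likely audio, and turns on the Smoke component for a few seconds before deactivating it.
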(event `self.Box.OnComponentBeginOverlap`
  (params (OverlappedComponent :type "PrimitiveComponent Object Reference") (OtherActor :type "Actor Object Reference") (OtherComp :type "PrimitiveComponent Object Reference") (OtherBodyIndex :type Integer) (bFromSweep :type Boolean) (SweepResult :type "HitResult Structure (by ref)"))
  (bind _asturtle_bp (cast `/Game/Blueprints/Turtle/Turtle_BP` OtherActor))
  (`KismetSystemLibrary.Delay` 1.2)
  (`self.K2_DestroyActor` _asturtle_bp)
  (`KismetSystemLibrary.Delay` 1.0)
  (`AudioComponent.Play` (`self.Burn`) 0.0)
  (`ActorComponent.Activate` (`self.Smoke`) false)
  (`KismetSystemLibrary.Delay` 5.0)
  (`ActorComponent.Deactivate` (`self.Smoke`)))

(fn `UserConstructionScript`)