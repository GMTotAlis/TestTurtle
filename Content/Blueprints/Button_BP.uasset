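; Numbered interactable button that spawns a turtle from the spawner with the matching number.
; On BeginPlay it displays its value plus one; Interact plays Press, changes the cylinder material and searches all Turtle_Spawner_BP actors for a match.
; After spawning, a delay restores the material and re-arms the button, with IsActive blocking repeat presses meanwhile.
; GetSelect supplies its selection text.
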(event `self.ReceiveBeginPlay`
  ;[1 1 1] Set number of Button when Game started
  (`TextRenderComponent.K2_SetText` (`self.Num Of Butt`) (`KismetTextLibrary.Conv_IntToText` (+ (`self.Button Value`) 1))))

(event `/Game/Blueprints/Interact_Interface_BP.Interact`
  (params (Player :type "Character Object Reference"))
  ;[1 1 1] Event when pressed E key
  (if (not (`self.Is Active`))
    (`AudioComponent.Play` (`self.Press`) 0.0)
    (set `self.Is Active` true)
    (`PrimitiveComponent.SetMaterial` (`self.Cylinder`) 0 "/Game/Materials/Doors_M.Doors_M")
    ;;[1 1 1] Find the right Spawner
    (bind _outactors (`GameplayStatics.GetAllActorsOfClass` "/Game/Blueprints/Turtle/Turtle_Spawner_BP.Turtle_Spawner_BP_C"))
    (for _array_element _outactors :!label _label
      (if (== (`/Game/Blueprints/Turtle/Turtle_Spawner_BP.Number Of Turtle` _array_element) (`self.Button Value`))
        (`/Game/Blueprints/Turtle/Turtle_Spawner_BP.SpawnTurtle` _array_element)
        (`self.Break`)
        (`KismetSystemLibrary.Delay` 8.0)
        (`PrimitiveComponent.SetMaterial` (`self.Cylinder`) 0 "/Game/Materials/Experiment_Wall_Angle_M.Experiment_Wall_Angle_M")
        (set `self.Is Active` false)))))

(event `Break`
  ;[1 1 1] Event when pressed E key
  ;;[1 1 1] Find the right Spawner
  (goto _label :!via `Break`))

(fn `Get Select`
  (returns (`Selected Button` :type Text))
  (return (`self.Selected Button Text`)))

(fn `UserConstructionScript`)